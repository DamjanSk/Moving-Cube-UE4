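; Door actor that swings open while the player pawn is inside its Trigger volume and makes the player's Cube disappear at a Teleport volume.
; Tick eases the door yaw toward open or closed by lerping from the current rotation, based on a per-frame overlap check.
; A Teleport overlap clears the Ready flag and calls EventDisappear on the Cube pawn.
; The older timeline-driven open and close logic is disconnected.
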(event `self.ReceiveTick`
  (params (DeltaSeconds :type "Float (single-precision)"))
  ;[1 1 1] Open / Close Door v2
  (`SceneComponent.K2_SetRelativeRotation` (`self.Door`) (`KismetMathLibrary.MakeRotator` (.roll (`SceneComponent.RelativeRotation` (`self.Door`))) (.pitch (`SceneComponent.RelativeRotation` (`self.Door`))) (`KismetMathLibrary.Lerp` (.yaw (`SceneComponent.RelativeRotation` (`self.Door`))) (`KismetMathLibrary.SelectFloat` 90.0 0.0 (`PrimitiveComponent.IsOverlappingActor` (`self.Trigger`) (`GameplayStatics.GetPlayerPawn` 0))) 0.05)) false false))

(event `self.Trigger.OnComponentEndOverlap`
  (params (OverlappedComponent :type "PrimitiveComponent Object Reference") (OtherActor :type "Actor Object Reference") (OtherComp :type "PrimitiveComponent Object Reference") (OtherBodyIndex :type Integer))
  ;[1 1 1] Close Door
)

(event `self.Trigger.OnComponentBeginOverlap`
  (params (OverlappedComponent :type "PrimitiveComponent Object Reference") (OtherActor :type "Actor Object Reference") (OtherComp :type "PrimitiveComponent Object Reference") (OtherBodyIndex :type Integer) (bFromSweep :type Boolean) (SweepResult :type "HitResult Structure (by ref)"))
  ;[1 1 1] Open door
)

(event `self.Teleport.OnComponentBeginOverlap`
  (params (OverlappedComponent :type "PrimitiveComponent Object Reference") (OtherActor :type "Actor Object Reference") (OtherComp :type "PrimitiveComponent Object Reference") (OtherBodyIndex :type Integer) (bFromSweep :type Boolean) (SweepResult :type "HitResult Structure (by ref)"))
  ;[1 1 1] Shrink Player
  (`self.If actor is player` OtherActor OtherComp)
  (if (`self.Ready`)
    (set `self.Ready` false)
    (bind _ascube (cast `/Game/Blueprints/Cube` (`GameplayStatics.GetPlayerPawn` 0)))
    (`/Game/Blueprints/Cube.Event Disappear` _ascube)))

(fn `If actor is player`
  (params (Actor :type "Object Object Reference") (Component :type "Object Object Reference"))
  (cast `StaticMeshComponent` Component)
  (if (== Actor (`GameplayStatics.GetPlayerPawn` 0))
    _))

(fn `UserConstructionScript`)